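; Gameplay game mode that sets up local multiplayer on BeginPlay, with game-only input and a hidden cursor.
; It loops over all PlayerStarts: the "Player1" tag uses controller 0, while every other start creates a new local player.
; Each controller gets its own Enhanced Input mapping context and possesses its own character class spawned at that start.
; An older index-based spawn loop remains in the graph but is unconnected.
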(event EventTick
  (params (DeltaSeconds :type Float%20%28single-precision%29)))

(event EventBeginPlay
  (bind _returnvalue (Game|GetPlayerController 0))
  (Variables|/Script/Engine.PlayerController|SetbShowMouseCursor _returnvalue false)
  (Input|SetInputModeGameOnly _returnvalue false)
  (bind _outactors (Actor|GetAllActorsOfClass "/Script/Engine.PlayerStart"))
  (for _array_element _outactors
    (if (== (Variables|/Script/Engine.PlayerStart|GetPlayerStartTag _array_element) "Player1")
      (bind _output_get (Variables|Default|SetPlayer1Controller (Game|GetPlayerController 0)))
      (Input|AddMappingContext (PlayerController|LocalPlayerSubsystems|GetEnhancedInputLocalPlayerSubsystem _output_get) "/Game/Blueprint/Input/Player1/IMC_Player1.IMC_Player1" 0 "(bIgnoreAllPressedKeysUntilRelease=True,bForceImmediately=False,bNotifyUserSettings=False)")
      (bind _returnvalue_2 (Game|SpawnActorfromClass "/Game/Blueprint/Character/BP_LocalMultiplayerCharacter1.BP_LocalMultiplayerCharacter1_C" (Transformation|GetActorTransform _array_element) "Undefined" "MultiplyWithRoot" 0 0))
      (Pawn|Possess (Variables|Default|GetPlayer1Controller) _returnvalue_2)
      (else
        (bind _returnvalue_3 (Class|GameplayStatics|CreatePlayer -1))
        (bind _output_get_2 (Variables|Default|SetPlayer2Controller _returnvalue_3))
        (Input|AddMappingContext (PlayerController|LocalPlayerSubsystems|GetEnhancedInputLocalPlayerSubsystem _output_get_2) "/Game/Blueprint/Input/Player2/IMC_Player2.IMC_Player2" 0 "(bIgnoreAllPressedKeysUntilRelease=True,bForceImmediately=False,bNotifyUserSettings=False)")
        (bind _returnvalue_4 (Game|SpawnActorfromClass "/Game/Blueprint/Character/BP_LocalMultiplayerCharacter2.BP_LocalMultiplayerCharacter2_C" (Transformation|GetActorTransform _array_element) "Undefined" "MultiplyWithRoot" 0 0))
        (Pawn|Possess (Variables|Default|GetPlayer2Controller) _returnvalue_4)))))

(fn ConstructionScript)